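; Purchasable inventory pickup for food, drinks and quest documents, with an interact prompt and price widget.
; The construction script uses PickupType to pick a preset mesh, name, class, icon and stacking, then packs them into ItemData.
; Radius overlaps register it with the ALS character; Interaction passes ItemData to the interactor, deducts the price and destroys it, checking only that player money exceeds zero.
; BeginPlay fills both widgets and toggles mesh physics after class-based delays.
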(event OnComponentBeginOverlap(Radius)
  (params (OverlappedComponent :type Primitive%20Component%20Object%20Reference) (OtherActor :type Actor%20Object%20Reference) (OtherComp :type Primitive%20Component%20Object%20Reference) (OtherBodyIndex :type Integer) (bFromSweep :type Boolean) (SweepResult :type Hit%20Result%20Structure%20%28by%20ref%29))
  (bind _asals_base_character (Utilities|Casting|CastToALS_BaseCharacter OtherActor))
  (Class|InterfaceBP|RegisterInteract(Message) _asals_base_character self))

(event OnComponentEndOverlap(Radius)
  (params (OverlappedComponent :type Primitive%20Component%20Object%20Reference) (OtherActor :type Actor%20Object%20Reference) (OtherComp :type Primitive%20Component%20Object%20Reference) (OtherBodyIndex :type Integer))
  (bind _asals_base_character (Utilities|Casting|CastToALS_BaseCharacter OtherActor))
  (Class|InterfaceBP|UnRegisterInteract(Message) _asals_base_character self))

(event EventBeginPlay
  (bind _pickupclass (Variables|Default|GetPickupClass))
  (Utilities|FlowControl|Sequence
    (:then_0
      (bind _asinteract_ui (Utilities|Casting|CastToInteractUI (UserInterface|GetUserWidgetObject (Variables|Default|GetUI))))
      (bind _output_get (Variables|Default|SetUIText _asinteract_ui))
      (Default|SetText _output_get (Variables|Default|GetTextPickUP))
      (Utilities|FlowControl|Sequence
        (:then_0
          (if (== _pickupclass "/Game/Inventory/Item/HealPickup.HealPickup_C")
            (Utilities|FlowControl|Delay 0.2 :!label _label)
            (Physics|SetSimulatePhysics (Variables|Default|GetMesh) true)
            (else
              (Utilities|FlowControl|Delay 5.0 :!label _label_2)
              (Physics|SetSimulatePhysics (Variables|Default|GetMesh) false))))
        (:then_1
          (if (== _pickupclass "/Game/Inventory/Item/StaminaPickup.StaminaPickup_C")
            (goto _label)
            (else
              (goto _label_2))))))
    (:then_1
      (bind _asharga (Utilities|Casting|CastToHarga (UserInterface|GetUserWidgetObject (Variables|Default|GetHarga))))
      (bind _output_get_2 (Variables|Default|SetUIHarga _asharga))
      (Default|SetHarga _output_get_2 (Utilities|Text|ToText(Integer) (Variables|Default|GetUang))))
    (:then_2
      (bind _asals_base_character (Utilities|Casting|CastToALS_BaseCharacter (Game|GetPlayerCharacter 0)))
      (Variables|Default|SetPlayer _asals_base_character))))

(event EventTick
  (params (DeltaSeconds :type Float%20%28single-precision%29)))

(event EventInteraction
  (params (Infestigator :type ALS%20Base%20Character%20Object%20Reference))
  (bind _itemdata (Variables|Default|GetItemData))
  (bind _player (Variables|Default|GetPlayer))
  (if (not (<= (Variables|/Game/AdvancedLocomotionV3/Blueprints/ALS_BaseCharacter.ALS_BaseCharacter_C|GetUang (Variables|Default|GetPlayer)) 0))
    (Default|Pickup Infestigator (Utilities|Struct|MakeItemStructure (.pickuptype _itemdata) (.pickupclass _itemdata) (.pickupname _itemdata) (.pickupactortext _itemdata) (.pickupimage _itemdata) (.canstack _itemdata) (+ (.quantity _itemdata) (Variables|Default|GetAmountToAdd))))
    (Variables|/Game/AdvancedLocomotionV3/Blueprints/ALS_BaseCharacter.ALS_BaseCharacter_C|SetUang _player (- (Variables|/Game/AdvancedLocomotionV3/Blueprints/ALS_BaseCharacter.ALS_BaseCharacter_C|GetUang _player) (Variables|Default|GetUang)))
    (Actor|DestroyActor)))

(fn ConstructionScript
  (CallFunction|SetRadius)
  (CallFunction|SetUILOC)
  (switch Utilities|FlowControl|Switch|SwitchonItemEnum (Variables|Default|GetPickupType)
    (:NewEnumerator0
      (|setRotiBulat))
    (:NewEnumerator1
      (|SusuCoklat))
    (:NewEnumerator2
      (|setKueCitron))
    (:NewEnumerator3
      (|setSusu))
    (:NewEnumerator4
      (|setMonsterEnergy))
    (:NewEnumerator5
      (|setRotiPanjang))
    (:NewEnumerator6
      (|SetRotiLapis))
    (:NewEnumerator7
      (|setPepsi))
    (:NewEnumerator8
      (|SetProposal))
    (:NewEnumerator9
      (|SetLaporan))
    (:NewEnumerator10
      (|SetPembayaran))
    (:NewEnumerator11
      (|SetPembayaranFotocopy))
    (:NewEnumerator12
      (|SetPembayaranFotocopy_2)))
  (Variables|Default|SetItemData (Utilities|Struct|MakeItemStructure (Variables|Default|GetPickupType) (Variables|Default|GetPickupClass) (Variables|Default|GetPickupName) (Variables|Default|GetPickupActorText) (Variables|Default|GetPickupImage) (Variables|Default|GetcanStack) (Variables|Default|GetQuantity))))

(fn SetHighlight
  (params (Hightlight :type Boolean))
  (Rendering|SetRenderCustomDepth (Variables|Default|GetMesh) Hightlight))

(fn SetRadius
  (bind _radius (Variables|Default|GetRadius))
  (Components|Sphere|SetSphereRadius _radius (Variables|Default|GetSetTriggerRadius) true)
  (Transformation|SetRelativeLocation _radius (Variables|Default|GetLocationTrigger) false false))

(fn SetUI
  (params (Visible :type Boolean))
  (Rendering|SetVisibility (Variables|Default|GetUI) Visible false))

(fn SetUILOC
  (Transformation|SetRelativeLocation (Variables|Default|GetUI) (Variables|Default|GetLocationUI) false false))

(fn SetHarga
  (params (Visible :type Boolean))
  (Rendering|SetVisibility (Variables|Default|GetHarga) Visible false))